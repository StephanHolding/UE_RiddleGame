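; Door actor that swings open and acts as a level exit, reloading the current level when the player walks through.
; OpenDoor sets an opened flag and plays a timeline that yaws the door mesh up to 90 degrees; CloseDoor reverses that timeline without clearing the flag.
; The box trigger's overlap reopens the current level by name only if the flag is set and the player pawn overlaps.
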(event OnComponentBeginOverlap(Box)
  (params (OverlappedComponent :type Primitive%20Component%20Object%20Reference) (OtherActor :type Actor%20Object%20Reference) (OtherComp :type Primitive%20Component%20Object%20Reference) (OtherBodyIndex :type Integer) (bFromSweep :type Boolean) (SweepResult :type Hit%20Result%20Structure%20%28by%20ref%29))
  (bind _returnvalue (Game|Player|GetPlayerPawn 0))
  (bind _returnvalue_2 (== OtherActor _returnvalue))
  (if (Variables|Default|GetdoorOpened)
    (if _returnvalue_2
      (Class|ScreenLogger|Log (Utilities|String|ToString(Boolean) _returnvalue_2))
      (bind _returnvalue_3 (Game|GetCurrentLevelName true))
      (Game|OpenLevel(byName) (Utilities|String|StringToName _returnvalue_3)))))

(event Custom|OpenDoor
  (Variables|Default|SetdoorOpened true)
  (bind _doorrotation (Timeline|DoorOpening Play)
    (:Update
      (Transformation|SetRelativeRotation (Variables|Default|GetMesh_Door_02) (Math|Rotator|MakeRotator 0.0 0.0 (Math|Float|Lerp 0.0 9e+01 _doorrotation)) false false))))

(event Custom|CloseDoor
  (bind _doorrotation (Timeline|DoorOpening Reverse)
    (:Update
      (Transformation|SetRelativeRotation (Variables|Default|GetMesh_Door_02) (Math|Rotator|MakeRotator 0.0 0.0 (Math|Float|Lerp 0.0 9e+01 _doorrotation)) false false))))

(fn ConstructionScript)