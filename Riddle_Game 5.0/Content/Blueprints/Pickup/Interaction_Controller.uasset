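; Interaction controller actor that lets its parent actor interact with Interactable components and hold Pickupables.
; Pickup input releases any held object, otherwise interacts using the selected mode, sphere overlap or camera raycast.
; Overlap picks through GetClosestInteractable, whose comparison actually favors the farthest candidate.
; Raycast hits only PhysicsBody objects and draws a debug line, with its endpoint not offset by camera location.
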(event Input|ActionEvents|InputActionPickup
  (params (Key :type Key%20Structure :default "None"))
  (:Pressed
    (if (== (Variables|Default|GetHoldingObject) 0)
      (switch Utilities|FlowControl|Switch|SwitchonInteractionMode (Variables|Default|GetinteractionMode)
        (:NewEnumerator0
          (CallFunction|TryInteractOverlap))
        (:NewEnumerator1
          (CallFunction|TryInteractRaycast)))
      (else
        (CallFunction|TryDeinteract)))))

(fn ConstructionScript)

(fn GetClosestInteractable
  (params (Interactable%20Components :type Array%20of%20Interactable%20Object%20References))
  (LocalVariables|SetclosestDistance 0.0)
  (if (> (Utilities|Array|Length Interactable%20Components) 0)
    (for (_array_element _array_index) Interactable%20Components
      (if (> (Transformation|GetDistanceTo (Components|GetOwner _array_element)) (LocalVariables|GetclosestDistance))
        (LocalVariables|SetclosestDistance (Transformation|GetDistanceTo (Components|GetOwner _array_element)))
        (LocalVariables|SetclosestComponentIndex _array_index)))
    (return (Utilities|Array|Get(acopy) Interactable%20Components (LocalVariables|GetclosestComponentIndex)))))

(fn TryInteractOverlap
  (bind _sphere (Variables|Default|GetSphere))
  (bind (_outactors _returnvalue) (Collision|ComponentOverlapActors _sphere (Transformation|GetWorldTransform _sphere) (Utilities|Array|MakeArray "ObjectTypeQuery3" "ObjectTypeQuery1" "ObjectTypeQuery2" "ObjectTypeQuery4") 0))
  (if _returnvalue
    (for _array_element _outactors
      (if (!= (Actor|GetComponentbyClass _array_element "/Game/Blueprints/Pickup/Interactable.Interactable_C") 0)
        (Utilities|Array|Add (LocalVariables|GetInteractableComponents) (Actor|GetComponentbyClass _array_element "/Game/Blueprints/Pickup/Interactable.Interactable_C"))))
    (if (> (Utilities|Array|Length (LocalVariables|GetInteractableComponents)) 0)
      (bind _closest_interactable (CallFunction|GetClosestInteractable (LocalVariables|GetInteractableComponents)))
      (bind _successful (Default|Interact _closest_interactable self))
      (if _successful
        (bind _aspickupable (Utilities|Casting|CastToPickupable _closest_interactable))
        (Variables|Default|SetHoldingObject _aspickupable)
        (else
          (Class|ScreenLogger|LogError "Interaction was unsuccesful!")))
      (else
        (Class|ScreenLogger|LogWarning "No Components found")))))

(fn TryDeinteract
  (bind _successful (Default|Deinteract (Variables|Default|GetHoldingObject) self))
  (if _successful
    (Variables|Default|SetHoldingObject 0)
    (else
      (Class|ScreenLogger|LogError "Deinteraction  was unssuccessful"))))

(fn TryInteractRaycast
  (bind _returnvalue (Actor|GetAttachParentActor))
  (bind _returnvalue_2 (Actor|GetComponentbyClass _returnvalue "/Script/Engine.CameraComponent"))
  (bind _returnvalue_3 (Transformation|GetWorldTransform _returnvalue_2))
  (bind (_location _rotation) (Math|Transform|BreakTransform _returnvalue_3))
  (bind _returnvalue_4 (Math|Vector|GetForwardVector _rotation))
  (bind _returnvalue_5 (* _returnvalue_4 1e+04))
  (Rendering|Debug|DrawDebugLine _location _returnvalue_5 "(R=0.092374,G=0.860133,B=1.000000,A=1.000000)" 1.0 1.0)
  (bind (_outhit _returnvalue_6) (Collision|LineTraceForObjects _location _returnvalue_5 (Utilities|Array|MakeArray "ObjectTypeQuery4") false 0 "None"))
  (if _returnvalue_6
    (if (!= (Actor|GetComponentbyClass (.HitActor (Collision|BreakHitResult _outhit)) "/Game/Blueprints/Pickup/Interactable.Interactable_C") 0)
      (bind _successful (Default|Interact (Actor|GetComponentbyClass (.HitActor (Collision|BreakHitResult _outhit)) "/Game/Blueprints/Pickup/Interactable.Interactable_C") self))
      (if _successful
        (bind _aspickupable (Utilities|Casting|CastToPickupable (Actor|GetComponentbyClass (.HitActor (Collision|BreakHitResult _outhit)) "/Game/Blueprints/Pickup/Interactable.Interactable_C")))
        (Variables|Default|SetHoldingObject _aspickupable)))))