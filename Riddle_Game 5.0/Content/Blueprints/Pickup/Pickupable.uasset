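; Component that lets its owning actor be picked up and dropped through the interaction system.
; Interact calls Pickup, which snaps the owner to the InteractionController's AttachmentPoint while keeping relative scale, then disables physics simulation and actor collision.
; Deinteract calls Drop, which detaches the owner with keep-relative rules and re-enables physics on its primitive component along with actor collision.
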(event EventBeginPlay)

(event EventTick
  (params (DeltaSeconds :type Float%20%28single-precision%29)))

(fn Pickup
  (params (interaction%20Controller :type Interaction%20Controller%20Object%20Reference))
  (bind _returnvalue (Components|GetOwner))
  (Transformation|AttachComponentToComponent _returnvalue (Variables|/Game/Blueprints/Pickup/Interaction_Controller.Interaction_Controller_C|GetAttachment%20Point interaction%20Controller) "None" "SnapToTarget" "SnapToTarget" "KeepRelative" true)
  (Physics|SetSimulatePhysics (Actor|GetComponentbyClass (Components|GetOwner) "/Script/Engine.PrimitiveComponent") false)
  (Collision|SetActorEnableCollision _returnvalue false))

(fn Drop
  (bind _returnvalue (Components|GetOwner))
  (Transformation|DetachFromActor _returnvalue "KeepRelative" "KeepRelative" "KeepRelative")
  (Physics|SetSimulatePhysics (Actor|GetComponentbyClass _returnvalue "/Script/Engine.PrimitiveComponent") true)
  (Collision|SetActorEnableCollision _returnvalue true))

(fn Interact
  (params (interaction_Controller :type Interaction%20Controller%20Object%20Reference))
  (CallFunction|Pickup interaction_Controller)
  (return true))

(fn Deinteract
  (params (interaction_Controller :type Interaction%20Controller%20Object%20Reference))
  (CallFunction|Drop)
  (return true))