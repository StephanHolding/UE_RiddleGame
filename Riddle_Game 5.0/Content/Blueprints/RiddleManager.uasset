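; Riddle manager for a timed puzzle room where bringing the right answer object into a trigger box opens a door.
; BeginPlay picks a random riddle from a data table, shows it on the Explanation widget and starts a one-second countdown that ends in a Game Over screen.
; Trigger overlaps compare the object's answer string to the riddle's and show feedback; a correct answer leaves the timer running.
; A helper spawns answer objects at random points but is not called here.
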(event OnComponentBeginOverlap(TriggerBox)
  (params (OverlappedComponent :type Primitive%20Component%20Object%20Reference) (OtherActor :type Actor%20Object%20Reference) (OtherComp :type Primitive%20Component%20Object%20Reference) (OtherBodyIndex :type Integer) (bFromSweep :type Boolean) (SweepResult :type Hit%20Result%20Structure%20%28by%20ref%29))
  (bind _aspossible_riddle_answer_object (Utilities|Casting|CastToPossibleRiddleAnswerObject OtherActor)
    (:then
      (if (!= _aspossible_riddle_answer_object 0)
        (if (Utilities|Enum|Equal(Enum) (Variables|/Game/Blueprints/PossibleRiddleAnswerObject.PossibleRiddleAnswerObject_C|GetriddleAnswerString _aspossible_riddle_answer_object) (.AnswerObjectName (Utilities|Struct|BreakFRiddleData (Variables|Default|GetcurrentRiddle))))
          (bind _asriddle_explanation (Utilities|Casting|CastToRiddleExplanation (UserInterface|GetWidget (Variables|Default|GetExplanation))))
          (Default|ApplyHintText _asriddle_explanation "That is correct!")
          (Class|ScreenLogger|Log "Correct!")
          (Default|OpenDoor (Variables|Default|GetDoor))
          (else
            (bind _asriddle_explanation_2 (Utilities|Casting|CastToRiddleExplanation (UserInterface|GetWidget (Variables|Default|GetExplanation))))
            (Default|ApplyHintText _asriddle_explanation_2 "That is incorrect.")
            (Class|ScreenLogger|LogWarning "Incorrect")))))
    (:CastFailed
      (Class|ScreenLogger|Log))))

(event EventBeginPlay
  (CallFunction|StartNewRiddle))

(fn ConstructionScript)

(fn SpawnAllPossibleAnswerObjects
  (bind _keys (Utilities|Map|Keys (Variables|AnswerObjects|GetspawnableObjectSettings)))
  (for _array_element _keys
    (bind _returnvalue (Game|SpawnActorfromClass "/Game/Blueprints/PossibleRiddleAnswerObject.PossibleRiddleAnswerObject_C" (Transformation|GetActorTransform (.OutItem (Utilities|Array|Random (Variables|AnswerObjects|GetallObjectSpawnTransforms)))) "Undefined" 0 0))
    (Default|ApplySettings _returnvalue (.Value (Utilities|Map|Find (Variables|AnswerObjects|GetspawnableObjectSettings) _array_element)))))

(fn StartNewRiddle
  (bind _outrownames (DataTable|GetDataTableRowNames "/Game/Resources/Riddles/Riddles.Riddles"))
  (bind _returnvalue (Utilities|GetDataTableRow "/Game/Resources/Riddles/Riddles.Riddles" (.OutItem (Utilities|Array|Random _outrownames)))
    (:then
      (bind _output_get (Variables|Default|SetcurrentRiddle _returnvalue))
      (Development|PrintString (.Question (Utilities|Struct|BreakFRiddleData _output_get)))
      (Development|PrintString (.Answer (Utilities|Struct|BreakFRiddleData _output_get)))
      (bind _asriddle_explanation (Utilities|Casting|CastToRiddleExplanation (UserInterface|GetWidget (Variables|Default|GetExplanation))))
      (Default|ApplyRiddleText _asriddle_explanation (.Question (Utilities|Struct|BreakFRiddleData _output_get)))
      (CallFunction|StartTimer))
    (:RowNotFound
      (Development|PrintString "Error!"))))

(fn StartTimer
  (Variables|Default|SetcurrentSeconds (Variables|Default|GetriddleSolveTimeInSeconds))
  (Utilities|Time|SetTimerbyFunctionName 0 "SecondElapsed" 1.0 (Variables|Default|GetloopTimer)))

(fn SecondElapsed
  (bind _result (Math|Integer|DecrementInt (Variables|Default|GetcurrentSeconds))
    (:%20%20
      (bind _asriddle_explanation (Utilities|Casting|CastToRiddleExplanation (UserInterface|GetWidget (Variables|Default|GetExplanation))))
      (Default|ApplyTimerText _asriddle_explanation (Utilities|String|Append (Utilities|String|ToString(Text) (Utilities|Text|ToText(Integer) (/ _result 60) false true 2)) ":" (Utilities|String|ToString(Text) (Utilities|Text|ToText(Integer) (- (Variables|Default|GetcurrentSeconds) (* (/ _result 60) 60)) false true 2))))
      (if (== (Variables|Default|GetcurrentSeconds) 0)
        (CallFunction|NoTimeLeft)))))

(fn NoTimeLeft
  (bind _returnvalue (Game|GetPlayerController 0))
  (Variables|Default|SetloopTimer false)
  (Class|KismetSystemLibrary|PauseTimer 0 "SecondElapsed")
  (Variables|/Script/Engine.PlayerController|SetbShowMouseCursor _returnvalue true)
  (bind _returnvalue_2 (UserInterface|CreateWidget "/Game/Blueprints/User_Interface/GameOver.GameOver_C"))
  (UserInterface|Viewport|AddtoViewport _returnvalue_2 0)
  (Input|SetInputModeGameandUI _returnvalue _returnvalue_2 "DoNotLock" false)
  (Class|CustomFunctionLibrary|CenterCursor _returnvalue))