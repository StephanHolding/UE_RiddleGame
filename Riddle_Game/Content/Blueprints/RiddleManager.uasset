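; RiddleManager picks a random riddle from the Riddles data table on BeginPlay and displays its question, also printing question and answer.
; It spawns one PossibleRiddleAnswerObject per SpawnableObjectSettings entry at randomly chosen transforms, which can repeat, and applies that entry's settings.
; Overlapping TriggerBox with an answer object compares its answer string to the riddle's AnswerObjectName and only logs the result.
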(event OnComponentBeginOverlap(TriggerBox)
  (params (OverlappedComponent :type Primitive%20Component%20Object%20Reference) (OtherActor :type Actor%20Object%20Reference) (OtherComp :type Primitive%20Component%20Object%20Reference) (OtherBodyIndex :type Integer) (bFromSweep :type Boolean) (SweepResult :type Hit%20Result%20Structure%20%28by%20ref%29))
  (bind _aspossible_riddle_answer_object (Utilities|Casting|CastToPossibleRiddleAnswerObject OtherActor)
    (:then
      (if (!= _aspossible_riddle_answer_object 0)
        (if (Utilities|Enum|Equal(Enum) (Variables|/Game/Blueprints/PossibleRiddleAnswerObject.PossibleRiddleAnswerObject_C|GetriddleAnswerString _aspossible_riddle_answer_object) (.AnswerObjectName (Utilities|Struct|BreakFRiddleData (Variables|Default|GetcurrentRiddle))))
          (Class|ScreenLogger|Log "Correct!")
          (else
            (Class|ScreenLogger|LogWarning "Incorrect")))))
    (:CastFailed
      (Class|ScreenLogger|Log))))

(event EventBeginPlay
  (bind _outrownames (DataTable|GetDataTableRowNames "/Game/Resources/Riddles/Riddles.Riddles"))
  (bind _returnvalue (Utilities|GetDataTableRow "/Game/Resources/Riddles/Riddles.Riddles" (.OutItem (Utilities|Array|Random _outrownames)))
    (:then
      (bind _output_get (Variables|Default|SetcurrentRiddle _returnvalue))
      (Development|PrintString (.Question (Utilities|Struct|BreakFRiddleData _output_get)))
      (Development|PrintString (.Answer (Utilities|Struct|BreakFRiddleData _output_get)))
      (Rendering|Components|TextRender|SetText (Variables|Default|GetRiddle) (Utilities|Text|ToText(String) (.Question (Utilities|Struct|BreakFRiddleData _output_get))))
      (CallFunction|SpawnAllPossibleAnswerObjects))
    (:RowNotFound
      (Development|PrintString "Error!"))))

(fn ConstructionScript)

(fn SpawnAllPossibleAnswerObjects
  (bind _keys (Utilities|Map|Keys (Variables|AnswerObjects|GetspawnableObjectSettings)))
  (for _array_element _keys
    (bind _returnvalue (Game|SpawnActorfromClass "/Game/Blueprints/PossibleRiddleAnswerObject.PossibleRiddleAnswerObject_C" (Transformation|GetActorTransform (.OutItem (Utilities|Array|Random (Variables|AnswerObjects|GetallObjectSpawnTransforms)))) "Undefined" 0 0))
    (Default|ApplySettings _returnvalue (.Value (Utilities|Map|Find (Variables|AnswerObjects|GetspawnableObjectSettings) _array_element)))))