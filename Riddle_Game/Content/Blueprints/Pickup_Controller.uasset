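; Pickup controller Blueprint that toggles picking up and dropping actors on the Pickup input action.
; TryPickup gathers Pickupable components from actors overlapping its Sphere, snap-attaches the selected one's owner to itself and calls Pickup.
; GetClosestPickupable's comparison actually selects the farthest candidate, despite its name.
; TryDrop detaches the held actor, calls Drop and clears HoldingObject.
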(event Input|ActionEvents|InputActionPickup
  (params (Key :type Key%20Structure :default "None"))
  (:Pressed
    (if (== (Variables|Default|GetHoldingObject) 0)
      (CallFunction|TryPickup)
      (else
        (CallFunction|TryDrop)))))

(fn ConstructionScript)

(fn GetClosestPickupable
  (params (Pickupable%20Components :type Array%20of%20Actor%20Component%20Object%20References))
  (LocalVariables|SetclosestDistance 0.0)
  (if (> (Utilities|Array|Length Pickupable%20Components) 0)
    (for (_array_element _array_index) Pickupable%20Components
      (if (> (Transformation|GetDistanceTo (Components|GetOwner _array_element)) (LocalVariables|GetclosestDistance))
        (LocalVariables|SetclosestDistance (Transformation|GetDistanceTo (Components|GetOwner _array_element)))
        (LocalVariables|SetclosestComponentIndex _array_index)))
    (bind _aspickupable (Utilities|Casting|CastToPickupable (Utilities|Array|Get(acopy) Pickupable%20Components (LocalVariables|GetclosestComponentIndex))))
    (return _aspickupable)))

(fn TryPickup
  (bind _sphere (Variables|Default|GetSphere))
  (bind (_outactors _returnvalue) (Collision|ComponentOverlapActors _sphere (Transformation|GetWorldTransform _sphere) (Utilities|Array|MakeArray "ObjectTypeQuery3" "ObjectTypeQuery1" "ObjectTypeQuery2" "ObjectTypeQuery4") 0))
  (if _returnvalue
    (for _array_element _outactors
      (if (!= (Actor|GetComponentbyClass _array_element "/Game/Blueprints/Pickupable.Pickupable_C") 0)
        (Utilities|Array|Add (LocalVariables|GetpickupableComponents) (Actor|GetComponentbyClass _array_element "/Game/Blueprints/Pickupable.Pickupable_C"))))
    (if (> (Utilities|Array|Length (LocalVariables|GetpickupableComponents)) 0)
      (bind _closest_pickupable (CallFunction|GetClosestPickupable (LocalVariables|GetpickupableComponents)))
      (Transformation|AttachActorToActor (Components|GetOwner _closest_pickupable) (Components|GetOwner (Variables|Default|GetDefaultSceneRoot)) "None" "SnapToTarget" "SnapToTarget" "KeepRelative" true)
      (Default|Pickup _closest_pickupable)
      (Variables|Default|SetHoldingObject _closest_pickupable)
      (else
        (Development|PrintString "No Components found")))))

(fn TryDrop
  (Development|PrintString "Dropping...")
  (Transformation|DetachFromActor (Components|GetOwner (Variables|Default|GetHoldingObject)) "KeepRelative" "KeepRelative" "KeepRelative")
  (Default|Drop (Variables|Default|GetHoldingObject))
  (Variables|Default|SetHoldingObject 0))